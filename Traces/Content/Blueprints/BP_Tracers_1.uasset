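; BP_Tracers_1 is an actor that fires a debug line trace every tick, apparently as a tracing test.
; The trace runs on the Visibility channel from its Arrow component a short distance along the arrow's forward vector, drawn for a duration.
; The hit result drives nothing, as the print comparing the hit actor to another actor is disconnected.
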(event `self.ReceiveTick`
  (params (DeltaSeconds :type "Float (single-precision)"))
  (bind _arrow (`self.Arrow`))
  (bind _returnvalue (`SceneComponent.K2_GetComponentLocation` _arrow))
  (bind _outhit (`KismetSystemLibrary.LineTraceSingle` :`Start` _returnvalue :`End` (+ _returnvalue (* (`SceneComponent.GetForwardVector` _arrow) 400.0)) :`TraceChannel` "TraceTypeQuery1" :`DrawDebugType` "ForDuration")))

(fn `UserConstructionScript`)